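; Hero character Blueprint that lets the player press K to interact with the nearest nearby actor tagged Interactable.
; Tick polls for the key press, scans all tagged actors for the closest, and acts only if it is within range.
; The target's secondary tag picks the result: Turret shows a one-time victory screen with UI-only input, Lamp applies a full-heal Gameplay Effect through GAS, and Float raises the actor.
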(event EventTick
  (params (DeltaSeconds :type Float%20%28single-precision%29))
  (bind _returnvalue (Game|GetPlayerController 0))
  (if (Game|Player|WasInputKeyJustPressed (Game|GetPlayerController 0) "K")
    (Variables|Default|SetClosestDist 9999.0)
    (bind _outactors (Actor|GetAllActorswithTag "Interactable"))
    (for _array_element _outactors
      (if (< (Transformation|GetDistanceTo _array_element) (Variables|Default|GetClosestDist))
        (Variables|Default|SetClosestDist (Transformation|GetDistanceTo _array_element))
        (Variables|Default|SetClosestTarget _array_element)))
    (if (<= (Variables|Default|GetClosestDist) 6e+02)
      (if (Actor|ActorHasTag (Variables|Default|GetClosestTarget) "Turret")
        (Utilities|FlowControl|DoOnce false
          (:Completed
            (bind _returnvalue_2 (UserInterface|CreateWidget "/Game/Blueprint/Widget/WBP_VictoryScreen.WBP_VictoryScreen_C" _returnvalue))
            (UserInterface|Viewport|AddtoViewport _returnvalue_2 100)
            (Input|SetInputModeUIOnly _returnvalue _returnvalue_2 "DoNotLock" false)
            (Variables|/Script/Engine.PlayerController|SetbShowMouseCursor _returnvalue true)))
        (elif (Actor|ActorHasTag (Variables|Default|GetClosestTarget) "Lamp")
          (bind _returnvalue_3 (Spec|MakeSpecHandle(ByClass) "/Game/Blueprint/HeroCharacter/GE_HealFull.GE_HealFull_C" self self))
          (GameplayEffects|ApplyGameplayEffectSpecToSelf (Variables|Default|GetAbilitySystemComponent) _returnvalue_3)
          (elif (Actor|ActorHasTag (Variables|Default|GetClosestTarget) "Float")
            (Transformation|SetActorLocation (Variables|Default|GetClosestTarget) (+ (Transformation|GetActorLocation (Variables|Default|GetClosestTarget)) (Math|Vector|MakeVector 0.0 0.0 5e+02)) false false)))))))

(fn ConstructionScript)