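; Boss enemy Blueprint that hooks into an ARPG AI agent component and seeds patrol points for its behavior.
; BeginPlay binds to the agent's OnDecisionReady, prints the decision's reason, and writes PatrolA and PatrolB to the Blackboard, offset either side of the spawn location along world X.
; The decision event feeds back into the same bind-and-print chain, so it rebinds and prints the reason each time it fires.
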(event Custom|OnDecisionReady_Event
  (params (Decision :type ARPG%20Decision%20Structure%20%28by%20ref%29))
  (EventDispatchers|BindEventtoOnDecisionReady (Variables|Default|GetARPGAIAgent) (delegate Custom|OnDecisionReady_Event))
  (Development|PrintString (.Reason (Utilities|Struct|BreakARPGDecision Decision)) true true "(R=0.757558,G=0.232622,B=1.000000,A=1.000000)"))

(event EventBeginPlay
  (bind _returnvalue (AI|GetBlackboard 0))
  (Utilities|FlowControl|Sequence
    (:then_0
      (EventDispatchers|BindEventtoOnDecisionReady (Variables|Default|GetARPGAIAgent) (delegate Custom|OnDecisionReady_Event))
      (Development|PrintString (.Reason (Utilities|Struct|BreakARPGDecision (stale Custom|OnDecisionReady_Event Decision))) true true "(R=0.757558,G=0.232622,B=1.000000,A=1.000000)"))
    (:then_1
      (AI|Components|Blackboard|SetValueasVector _returnvalue (Utilities|Name|MakeLiteralName "PatrolA") (+ (Transformation|GetActorLocation) (Math|Vector|MakeVector 3e+02 0.0 0.0)))
      (AI|Components|Blackboard|SetValueasVector _returnvalue (Utilities|Name|MakeLiteralName "PatrolB") (+ (Transformation|GetActorLocation) (Math|Vector|MakeVector -3e+02 0.0 0.0))))))

(fn ConstructionScript)